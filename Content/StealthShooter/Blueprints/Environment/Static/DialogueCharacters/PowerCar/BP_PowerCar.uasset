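; BP_PowerCar is an interactable power car that plays a voice line and shows a dialogue widget that depends on whether the player holds the key item.
; On BeginPlay it finds BP_EndGameTrigger and disables its collision.
; Interacting with the item removes the car's smoke and sparks, sets ItemGained and re-enables the trigger as query-only.
; Leaving the interaction collision hides the widget.
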(event `self.ReceiveBeginPlay`
  (bind _asbp_ssgame_mode (cast `/Game/StealthShooter/Core/GameModes/BP_SSGameMode` (`GameplayStatics.GetGameMode`)))
  (set `self.SSGame Mode` _asbp_ssgame_mode)
  (bind _returnvalue (`GameplayStatics.GetActorOfClass` "/Game/StealthShooter/Blueprints/Environment/Static/Triggers/BP_EndGameTrigger.BP_EndGameTrigger_C"))
  (bind _output_get (set `self.EndGameTrigger` _returnvalue))
  (`PrimitiveComponent.SetCollisionEnabled` (`/Game/StealthShooter/Blueprints/Environment/Static/Triggers/BP_EndGameTrigger.Box` _output_get) "NoCollision"))

(event `/Game/StealthShooter/Blueprints/Interfaces/BPI_Interactable.Interact`
  (`SceneComponent.SetVisibility` (`self.Widget`) true false)
  (`GameplayStatics.PlaySoundAtLocation` "/Game/StealthShooter/FX/Sound/Cues/C_PowerCarVoice.C_PowerCarVoice" (`self.K2_GetActorLocation`) (struct) 1.0 1.0 0.0 null null null null)
  (if (`self.bPlayerHasKeyItem`)
    (`WidgetComponent.SetWidget` (`self.Widget`) (`self.WithItemWidget`))
    (bind _smoke (`self.Smoke`)
      (:`then`
        (`ActorComponent.K2_DestroyComponent` _smoke)
        (bind _sparks (`self.Sparks`)
          (:`then`
            (`ActorComponent.K2_DestroyComponent` _sparks)
            (set `self.bItemGained` true)
            (bind _endgametrigger (`self.EndGameTrigger`)
              (:`then`
                (`PrimitiveComponent.SetCollisionEnabled` (`/Game/StealthShooter/Blueprints/Environment/Static/Triggers/BP_EndGameTrigger.Box` _endgametrigger) "QueryOnly"))
              (:`else`)))
          (:`else`)))
      (:`else`))
    (else
      (`WidgetComponent.SetWidget` (`self.Widget`) (`self.WithoutItemWidget`)))))

(event `self.InteractCollision.OnComponentEndOverlap`
  (params (OverlappedComponent :type "PrimitiveComponent Object Reference") (OtherActor :type "Actor Object Reference") (OtherComp :type "PrimitiveComponent Object Reference") (OtherBodyIndex :type Integer))
  (`SceneComponent.SetVisibility` (`self.Widget`) false false))

(fn `UserConstructionScript`)