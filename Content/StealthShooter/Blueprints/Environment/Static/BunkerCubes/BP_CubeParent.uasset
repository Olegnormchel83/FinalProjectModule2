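; BP_CubeParent is the base Blueprint for static bunker cube props in the stealth shooter's environment.
; Its construction script applies a random entry from the Materials array to the first material slot, then picks the small, middle or large cube mesh from CubeSize.
; All setup happens at construction, with no active runtime logic in the event graph.
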(fn `UserConstructionScript`
  (bind _staticmesh (`self.StaticMesh`))
  (`|ExecutionSequence`
    (:`then_0`
      (`PrimitiveComponent.SetMaterial` (`self.StaticMesh`) 0 (`KismetArrayLibrary.Array_Random` (`self.Materials`))))
    (:`then_1`
      (switch `/Game/StealthShooter/Blueprints/Enums/E_CubeSize` (`self.CubeSize`)
        (:`NewEnumerator0`
          (`StaticMeshComponent.SetStaticMesh` _staticmesh "/Game/StealthShooter/ExternalMeshes/UGSciFi/SM_Cube_60cm.SM_Cube_60cm"))
        (:`NewEnumerator1`
          (`StaticMeshComponent.SetStaticMesh` _staticmesh "/Game/StealthShooter/ExternalMeshes/UGSciFi/SM_Cube_3m.SM_Cube_3m"))
        (:`NewEnumerator2`
          (`StaticMeshComponent.SetStaticMesh` _staticmesh "/Game/StealthShooter/ExternalMeshes/UGSciFi/SM_Cube_6m.SM_Cube_6m"))))))