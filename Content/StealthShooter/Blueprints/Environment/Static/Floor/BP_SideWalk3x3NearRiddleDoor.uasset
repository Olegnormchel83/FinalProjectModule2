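; BP_SideWalk3x3NearRiddleDoor is a 3x3 grid of sidewalk floor plates that stays hidden until revealed, placed near the riddle door.
; On BeginPlay it gathers the nine plate components into an array, hiding each and disabling its collision.
; The SetPlatesVisible event loops over that array to show every plate and restore query and physics collision.
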(event `self.ReceiveBeginPlay`
  (bind _output_get (set `self.Plates` (`|MakeArray` (`self.SideWalk1`) (`self.SideWalk2`) (`self.SideWalk3`) (`self.SideWalk4`) (`self.SideWalk5`) (`self.SideWalk6`) (`self.SideWalk7`) (`self.SideWalk8`) (`self.SideWalk9`))))
  (for _array_element _output_get
    (`SceneComponent.SetVisibility` _array_element false false)
    (`PrimitiveComponent.SetCollisionEnabled` _array_element "NoCollision")))

(event `SetPlatesVisible`
  (for _array_element (`self.Plates`)
    (`SceneComponent.SetVisibility` _array_element true false)
    (`PrimitiveComponent.SetCollisionEnabled` _array_element "QueryAndPhysics")))

(fn `UserConstructionScript`)