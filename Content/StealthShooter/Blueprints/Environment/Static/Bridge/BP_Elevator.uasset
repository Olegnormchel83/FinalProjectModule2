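; Bridge elevator actor that, on Interact, seals its entrance and carries itself up a fixed height before opening its exit.
; BeginPlay clears the entrance wall mesh and caches the game instance; Interact restores that wall as a glitch-material dead end and destroys the Box trigger.
; The ElevatorUp timeline maps its ZOffset track from the actor's current Z, re-read every update, toward the target height, then clears the exit wall mesh.
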(event `self.ReceiveBeginPlay`
  (`StaticMeshComponent.SetStaticMesh` (`self.CubeWall2Enter`) null)
  (bind _asbp_ssgame_instance (cast `/Game/StealthShooter/Core/GameInstance/BP_SSGameInstance` (`GameplayStatics.GetGameInstance`)))
  (set `self.SSGame Instance` _asbp_ssgame_instance))

(event `self.Box.OnComponentBeginOverlap`
  (params (OverlappedComponent :type "PrimitiveComponent Object Reference") (OtherActor :type "Actor Object Reference") (OtherComp :type "PrimitiveComponent Object Reference") (OtherBodyIndex :type Integer) (bFromSweep :type Boolean) (SweepResult :type "HitResult Structure (by ref)")))

(event `/Game/StealthShooter/Blueprints/Interfaces/BPI_Interactable.Interact`
  (bind (_returnvalue_x _returnvalue_y _returnvalue_z) (`KismetMathLibrary.BreakVector` (`self.K2_GetActorLocation`)))
  (bind (_returnvalue_x_2 _returnvalue_y_2 _returnvalue_z_2) (`KismetMathLibrary.BreakVector` (`self.K2_GetActorLocation`)))
  (bind _cubewall2enter (`self.CubeWall2Enter`))
  (`StaticMeshComponent.SetStaticMesh` _cubewall2enter "/Game/StealthShooter/ExternalMeshes/UGSciFi/SM_Bunker_Wall_Deadend.SM_Bunker_Wall_Deadend")
  (`PrimitiveComponent.SetMaterial` _cubewall2enter 0 "/Game/StealthShooter/ExternalMeshes/UGSciFi/Materials/Glitches/M_Glitch02.M_Glitch02")
  (set `self.TargetZOffset` (+ _returnvalue_z_2 1620.0))
  (`ActorComponent.K2_DestroyComponent` (`self.Box`))
  (bind (_direction _zoffset) (`Timeline|ElevatorUp` :`NewTime` 5.0 :!via `PlayFromStart`)
    (:`Update`
      (`self.K2_SetActorLocation` (`KismetMathLibrary.MakeVector` _returnvalue_x _returnvalue_y (`KismetMathLibrary.MapRangeClamped` _zoffset 0.0 100.0 _returnvalue_z (`self.TargetZOffset`)))))
    (:`Finished`
      (`StaticMeshComponent.SetStaticMesh` (`self.CubeWall1Exit`) null))))

(fn `UserConstructionScript`)