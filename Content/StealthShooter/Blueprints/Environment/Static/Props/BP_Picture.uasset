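; BP_Picture is a static environment prop that builds a randomized arrangement of pictures.
; Its construction script loops over nine picture mesh components, giving each a random visibility and a random static mesh from the Meshes array.
; The variation is rolled whenever the construction script runs, and the event graph holds no active gameplay logic.
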(fn `UserConstructionScript`
  (for _array_element (`|MakeArray` (`self.Pic1`) (`self.Pic2`) (`self.Pic3`) (`self.Pic4`) (`self.Pic5`) (`self.Pic6`) (`self.Pic7`) (`self.Pic8`) (`self.Pic9`))
    (`SceneComponent.SetVisibility` _array_element (`KismetMathLibrary.RandomBool`) false)
    (`StaticMeshComponent.SetStaticMesh` _array_element (`KismetArrayLibrary.Array_Random` (`self.Meshes`)))))