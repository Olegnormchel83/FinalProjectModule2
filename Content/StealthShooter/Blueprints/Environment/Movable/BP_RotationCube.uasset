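; BP_RotationCube is a movable environment cube that periodically tumbles to a new orientation on its own.
; A looping timer from BeginPlay fires RotationCube, which randomly picks a quarter or half turn and applies it to either roll or pitch.
; The SmoothRoatation timeline then lerps the actor from its current rotation to that target.
; Per-axis helper functions XRotation, YRotation and ZRotation also exist, but the event graph never calls them.
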(event `self.ReceiveBeginPlay`
  (bind _returnvalue (`KismetSystemLibrary.K2_SetTimerDelegate` (delegate `RotationCube`) (`self.TimeBetweenRotation`) true))
  (set `self.RotationTimerHandle` _returnvalue))

(event `RotationCube`
  (bind (_initialrotation_roll _initialrotation_pitch _initialrotation_yaw) (`KismetMathLibrary.BreakRotator` (`self.InitialRotation`)))
  (bind (_initialrotation_roll_2 _initialrotation_pitch_2 _initialrotation_yaw_2) (`KismetMathLibrary.BreakRotator` (`self.InitialRotation`)))
  (set `self.InitialRotation` (`self.K2_GetActorRotation`))
  (switch `int` (`KismetMathLibrary.RandomIntegerInRange` 0 1)
    (:`0`
      (set `self.RotationDegrees` 90.0))
    (:`1`
      (set `self.RotationDegrees` 180.0)))
  (switch `int` (`KismetMathLibrary.RandomIntegerInRange` 0 1)
    (:`0`
      (set `self.TargetRotation` (`KismetMathLibrary.MakeRotator` (+ _initialrotation_roll_2 (`self.RotationDegrees`)) _initialrotation_pitch_2 _initialrotation_yaw_2))
      (bind (_direction _rotation) (`Timeline|SmoothRoatation` :`NewTime` (/ 1.0 (`self.RotationSpeed`)) :!via `PlayFromStart` :!label _label)
        (:`Update`
          (`self.K2_SetActorRotation` (`KismetMathLibrary.RLerp` (`self.InitialRotation`) (`self.TargetRotation`) _rotation)))))
    (:`1`
      (set `self.TargetRotation` (`KismetMathLibrary.MakeRotator` _initialrotation_roll (+ _initialrotation_pitch (`self.RotationDegrees`)) _initialrotation_yaw))
      (goto _label :!via `PlayFromStart`))))

(fn `UserConstructionScript`)

(fn `XRotation`
  (params (RotationValue :type "Float (double-precision)"))
  (bind (_returnvalue_roll _returnvalue_pitch _returnvalue_yaw) (`KismetMathLibrary.BreakRotator` (`self.K2_GetActorRotation`)))
  (`SceneComponent.K2_SetWorldRotation` (`self.StaticMesh`) (`KismetMathLibrary.MakeRotator` (+ RotationValue _returnvalue_roll) _returnvalue_pitch _returnvalue_yaw) false false))

(fn `YRotation`
  (params (RotationValue :type "Float (double-precision)"))
  (bind (_returnvalue_roll _returnvalue_pitch _returnvalue_yaw) (`KismetMathLibrary.BreakRotator` (`self.K2_GetActorRotation`)))
  (`SceneComponent.K2_SetWorldRotation` (`self.StaticMesh`) (`KismetMathLibrary.MakeRotator` _returnvalue_roll (+ RotationValue _returnvalue_pitch) _returnvalue_yaw) false false))

(fn `ZRotation`
  (params (RotationValue :type "Float (double-precision)"))
  (bind (_returnvalue_roll _returnvalue_pitch _returnvalue_yaw) (`KismetMathLibrary.BreakRotator` (`self.K2_GetActorRotation`)))
  (`self.K2_SetActorRotation` (`KismetMathLibrary.MakeRotator` _returnvalue_roll _returnvalue_pitch (+ RotationValue _returnvalue_yaw))))