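; Proximity-triggered explosive hazard that starts a countdown when the player enters its trigger sphere, sized from Radius in the construction script.
; Overlap plays a tick sound and starts two timers: a delayed explosion and a looping blink that drives the point light's red channel through a timeline.
; The explosion applies radial damage at twice the trigger radius, blockable on a custom trace channel, spawns effects and destroys the actor.
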(event `self.ReceiveBeginPlay`
  (`parent.ReceiveBeginPlay`))

(event `self.Sphere.OnComponentBeginOverlap`
  (params (OverlappedComponent :type "PrimitiveComponent Object Reference") (OtherActor :type "Actor Object Reference") (OtherComp :type "PrimitiveComponent Object Reference") (OtherBodyIndex :type Integer) (bFromSweep :type Boolean) (SweepResult :type "HitResult Structure (by ref)"))
  (bind _isplayer (`self.IsPlayer` OtherActor))
  (if _isplayer
    (bind _returnvalue (`KismetSystemLibrary.K2_SetTimerDelegate` (delegate `Explode`) (`self.TimeToExplode`)))
    (set `self.ExplodeTimerHandle` _returnvalue)
    (`GameplayStatics.PlaySoundAtLocation` "/Game/StealthShooter/FX/Sound/Cues/C_BombTick.C_BombTick" (`self.K2_GetActorLocation`) (struct) 1.0 1.0 0.0 null null null null)
    (bind _returnvalue_2 (`KismetSystemLibrary.K2_SetTimerDelegate` (delegate `Blinking`) 0.5 true))
    (set `self.BlinkingTimerHandle` _returnvalue_2)))

(event `Blinking`
  (bind (_direction _blinktrack) (`Timeline|Timeline` :!via `PlayFromStart`)
    (:`Update`
      (`LightComponent.SetLightColor` (`self.PointLight`) (make `LinearColor` _blinktrack 0.0 0.0 1.0) true))))

(event `Explode`
  (bind _returnvalue (`self.K2_GetActorLocation`))
  (`GameplayStatics.ApplyRadialDamage` :`BaseDamage` (`self.Damage`) :`Origin` _returnvalue :`DamageRadius` (* (`self.Radius`) 2.0) :`DamageCauser` self :`InstigatedByController` null :`bDoFullDamage` (`self.DoFullDamage`) :`DamagePreventionChannel` "ECC_GameTraceChannel2")
  (`GameplayStatics.SpawnEmitterAtLocation` "/Game/StealthShooter/FX/Visual/P_Explosion.P_Explosion" _returnvalue)
  (`GameplayStatics.PlaySoundAtLocation` "/Game/StealthShooter/FX/Sound/Cues/c_Explosion.c_Explosion" _returnvalue (struct) 1.0 1.0 0.0 null null null null)
  (`KismetSystemLibrary.K2_ClearAndInvalidateTimerHandle` (`self.ExplodeTimerHandle`))
  (`KismetSystemLibrary.K2_ClearAndInvalidateTimerHandle` (`self.BlinkingTimerHandle`))
  (`self.K2_DestroyActor`))

(fn `UserConstructionScript`
  (`parent.UserConstructionScript`)
  (`SphereComponent.SetSphereRadius` (`self.Sphere`) (`self.Radius`) true))