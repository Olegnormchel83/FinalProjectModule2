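; BP_SmallFire is an environmental fire hazard that repeatedly damages the player while inside its sphere and plays a fire sound on BeginPlay.
; Player overlap starts a fast looping timer that applies Damage to the overlapping actor, and end overlap clears that timer.
; The construction script sizes the sphere from the Radius variable.
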(event `self.ReceiveBeginPlay`
  (`parent.ReceiveBeginPlay`)
  (`GameplayStatics.PlaySoundAtLocation` "/Game/StealthShooter/FX/Sound/Cues/C_Fire.C_Fire" (`self.K2_GetActorLocation`) (struct) 1.0 1.0 0.0 null null null null))

(event `self.Sphere.OnComponentBeginOverlap`
  (params (OverlappedComponent :type "PrimitiveComponent Object Reference") (OtherActor :type "Actor Object Reference") (OtherComp :type "PrimitiveComponent Object Reference") (OtherBodyIndex :type Integer) (bFromSweep :type Boolean) (SweepResult :type "HitResult Structure (by ref)"))
  (bind _isplayer (`self.IsPlayer` OtherActor))
  (if _isplayer
    (bind _returnvalue (`KismetSystemLibrary.K2_SetTimerDelegate` (delegate `Burning`) 0.1 true))
    (set `self.FireTimerHandle` _returnvalue)))

(event `Burning`
  (`GameplayStatics.ApplyDamage` (stale `self.Sphere.OnComponentBeginOverlap` OtherActor) (`self.Damage`) null self))

(event `self.Sphere.OnComponentEndOverlap`
  (params (OverlappedComponent :type "PrimitiveComponent Object Reference") (OtherActor :type "Actor Object Reference") (OtherComp :type "PrimitiveComponent Object Reference") (OtherBodyIndex :type Integer))
  (bind _isplayer (`self.IsPlayer` OtherActor))
  (if _isplayer
    (`KismetSystemLibrary.K2_ClearAndInvalidateTimerHandle` (`self.FireTimerHandle`))))

(fn `UserConstructionScript`
  (`parent.UserConstructionScript`)
  (`SphereComponent.SetSphereRadius` (`self.Sphere`) (`self.Radius`) true))