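; Base Blueprint for environment damage items in StealthShooter, with no damage logic of its own.
; BeginPlay calls DestroyComponent on the StaticMesh and ParticleSystem components when their IsValid checks fail, then caches the BP_SSGameInstance.
; IsPlayer uses that cached instance to test whether an actor carries the player tag, so the tag is defined centrally in the game instance.
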(event `self.ReceiveBeginPlay`
  (bind _staticmesh (`self.StaticMesh`))
  (bind _particlesystem (`self.ParticleSystem`))
  (`|ExecutionSequence`
    (:`then_0`
      (`/Engine/EditorBlueprintResources/StandardMacros.IsValid` _staticmesh
        (:`Is Not Valid`
          (`ActorComponent.K2_DestroyComponent` _staticmesh))))
    (:`then_1`
      (`/Engine/EditorBlueprintResources/StandardMacros.IsValid` _particlesystem
        (:`Is Not Valid`
          (`ActorComponent.K2_DestroyComponent` _particlesystem))))
    (:`then_2`
      (bind _asbp_ssgame_instance (cast `/Game/StealthShooter/Core/GameInstance/BP_SSGameInstance` (`GameplayStatics.GetGameInstance`)))
      (set `self.SSGame Instance` _asbp_ssgame_instance))))

(fn `IsPlayer`
  (params (InActor :type "Actor Object Reference"))
  (returns (IsPlayer :type Boolean))
  (bind _ssgame_instance (`self.SSGame Instance`)
    (:`then`
      (return (`self.ActorHasTag` InActor (`/Game/StealthShooter/Core/GameInstance/BP_SSGameInstance.GetPlayerTag` _ssgame_instance))))
    (:`else`)))

(fn `UserConstructionScript`)