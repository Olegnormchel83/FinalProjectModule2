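; BP_DoorParent is a base door Blueprint that opens permanently when the player approaches.
; A Box overlap checks for the player tag, the CanOpen flag and that opening has not already started, then calls OpenDoor.
; OpenDoor plays a sound and runs a timeline that slides the Door vertically along its relative Z.
; When the timeline finishes, both the Door and the trigger Box are destroyed, so it never closes.
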(event `OpenDoor`
  (bind _door (`self.Door`))
  (bind (_relativelocation_x _relativelocation_y) (`KismetMathLibrary.BreakVector` (`SceneComponent.RelativeLocation` _door)))
  (set `self.bIsAlreadyOpening` true)
  (`GameplayStatics.PlaySoundAtLocation` "/Game/StealthShooter/FX/Sound/Cues/C_OpenDoor.C_OpenDoor" (`self.K2_GetActorLocation`) (struct) 1.0 1.0 0.0 null null null null)
  (bind (_direction _zoffsetdoor) (`Timeline|OpenDoorTimeline` :!via `PlayFromStart`)
    (:`Update`
      (`SceneComponent.K2_SetRelativeLocation` _door (`KismetMathLibrary.MakeVector` _relativelocation_x _relativelocation_y _zoffsetdoor) false false))
    (:`Finished`
      (`ActorComponent.K2_DestroyComponent` (`self.Door`))
      (`ActorComponent.K2_DestroyComponent` (`self.Box`)))))

(event `self.Box.OnComponentBeginOverlap`
  (params (OverlappedComponent :type "PrimitiveComponent Object Reference") (OtherActor :type "Actor Object Reference") (OtherComp :type "PrimitiveComponent Object Reference") (OtherBodyIndex :type Integer) (bFromSweep :type Boolean) (SweepResult :type "HitResult Structure (by ref)"))
  (if (`self.ActorHasTag` OtherActor (`self.PlayerTag`))
    (if (`self.bCanOpen`)
      (if (not (`self.bIsAlreadyOpening`))
        (`self.OpenDoor`)))))

(fn `UserConstructionScript`)