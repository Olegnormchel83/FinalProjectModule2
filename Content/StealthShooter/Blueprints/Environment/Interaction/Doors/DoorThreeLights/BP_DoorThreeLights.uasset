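; Door Blueprint for a puzzle door that can open only when its three lights are all lit.
; On BeginPlay it binds a handler to the activation event of each of three referenced switches, skipping any that are invalid.
; CheckSolution reads the visibility of the three point lights and sets CanOpen true if all are visible, false otherwise.
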(event `self.ReceiveBeginPlay`
  (`|ExecutionSequence`
    (:`then_0`
      (bind _switch1 (`self.Switch1`)
        (:`then`
          (add `/Game/StealthShooter/Blueprints/Environment/Interaction/Doors/DoorThreeLights/BP_SwitchParent.SwitchActivated` _switch1 (`|CreateDelegate` :!event `CheckSolution`)))
        (:`else`)))
    (:`then_1`
      (bind _switch2 (`self.Switch2`)
        (:`then`
          (add `/Game/StealthShooter/Blueprints/Environment/Interaction/Doors/DoorThreeLights/BP_SwitchParent.SwitchActivated` _switch2 (`|CreateDelegate` :!event `CheckSolution`)))
        (:`else`)))
    (:`then_2`
      (bind _switch3 (`self.Switch3`)
        (:`then`
          (add `/Game/StealthShooter/Blueprints/Environment/Interaction/Doors/DoorThreeLights/BP_SwitchParent.SwitchActivated` _switch3 (`|CreateDelegate` :!event `CheckSolution`)))
        (:`else`)))))

(event `CheckSolution`
  (if (`SceneComponent.IsVisible` (`self.PointLight1`))
    (if (`SceneComponent.IsVisible` (`self.PointLight2`))
      (if (`SceneComponent.IsVisible` (`self.PointLight3`))
        (set `self.bCanOpen` true)
        (else
          (set `self.bCanOpen` false :!label _label)))
      (else
        (goto _label)))
    (else
      (goto _label))))

(fn `UserConstructionScript`
  (`parent.UserConstructionScript`))