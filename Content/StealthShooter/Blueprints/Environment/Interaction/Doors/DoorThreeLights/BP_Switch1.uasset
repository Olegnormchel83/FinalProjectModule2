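; Interactable switch, part of the three-light door setup, that toggles the first point light on its Target actor.
; On BeginPlay it caches the Target's PointLight1 and sets its text label to the on or off text based on that light's visibility.
; Each Interact flips the light's visibility, updates the label and fires the SwitchActivated dispatcher.
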(event `self.ReceiveBeginPlay`
  (bind _target (`self.Target`)
    (:`then`
      (bind _pointlight1 (`/Game/StealthShooter/Blueprints/Environment/Interaction/Doors/DoorThreeLights/BP_DoorThreeLights.PointLight1` _target)
        (:`then`
          (set `self.Point Light 1` _pointlight1)
          (if (`SceneComponent.IsVisible` _pointlight1)
            (`TextRenderComponent.K2_SetText` (`self.TextRender`) (`self.TextON`))
            (else
              (`TextRenderComponent.K2_SetText` (`self.TextRender`) (`self.TextOFF`)))))
        (:`else`)))
    (:`else`)))

(event `/Game/StealthShooter/Blueprints/Interfaces/BPI_Interactable.Interact`
  (bind _point_light_1 (`self.Point Light 1`)
    (:`then`
      (if (`SceneComponent.IsVisible` _point_light_1)
        (`SceneComponent.SetVisibility` _point_light_1 false false)
        (`TextRenderComponent.K2_SetText` (`self.TextRender`) (`self.TextOFF`))
        (else
          (`SceneComponent.SetVisibility` _point_light_1 true false)
          (`TextRenderComponent.K2_SetText` (`self.TextRender`) (`self.TextON`))))
      (`self.SwitchActivated`))
    (:`else`)))

(fn `UserConstructionScript`)