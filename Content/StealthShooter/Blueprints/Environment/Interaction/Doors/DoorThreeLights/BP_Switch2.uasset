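; BP_Switch2 is an interactable switch for the three-light door that toggles the second point light on its Target actor.
; On BeginPlay it caches the target's PointLight2 and sets its text label to match the light's visibility.
; Each Interact flips that visibility, updates the ON/OFF text and fires the SwitchActivated dispatcher.
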(event `self.ReceiveBeginPlay`
  (bind _target (`self.Target`)
    (:`then`
      (bind _pointlight2 (`/Game/StealthShooter/Blueprints/Environment/Interaction/Doors/DoorThreeLights/BP_DoorThreeLights.PointLight2` _target)
        (:`then`
          (set `self.Point Light2` _pointlight2)
          (if (`SceneComponent.IsVisible` _pointlight2)
            (`TextRenderComponent.K2_SetText` (`self.TextRender`) (`self.TextON`))
            (else
              (`TextRenderComponent.K2_SetText` (`self.TextRender`) (`self.TextOFF`)))))
        (:`else`)))
    (:`else`)))

(event `self.Interact`
  (bind _point_light2 (`self.Point Light2`)
    (:`then`
      (if (`SceneComponent.IsVisible` _point_light2)
        (`SceneComponent.SetVisibility` _point_light2 false false)
        (`TextRenderComponent.K2_SetText` (`self.TextRender`) (`self.TextOFF`))
        (else
          (`SceneComponent.SetVisibility` _point_light2 true false)
          (`TextRenderComponent.K2_SetText` (`self.TextRender`) (`self.TextON`))))
      (`self.SwitchActivated`))
    (:`else`)))

(fn `UserConstructionScript`)