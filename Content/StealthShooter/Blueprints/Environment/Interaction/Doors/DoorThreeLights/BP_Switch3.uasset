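; BP_Switch3 is an interactable switch, one part of the three-light door setup, that toggles the third point light on its Target.
; On BeginPlay it caches Target's PointLight3 and sets its text label to match whether the light is visible.
; Interact flips the light's visibility, updates the on/off label and fires the SwitchActivated dispatcher.
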(event `self.ReceiveBeginPlay`
  (bind _target (`self.Target`)
    (:`then`
      (bind _pointlight3 (`/Game/StealthShooter/Blueprints/Environment/Interaction/Doors/DoorThreeLights/BP_DoorThreeLights.PointLight3` _target)
        (:`then`
          (set `self.PointLight3` _pointlight3)
          (if (`SceneComponent.IsVisible` _pointlight3)
            (`TextRenderComponent.K2_SetText` (`self.TextRender`) (`self.TextON`))
            (else
              (`TextRenderComponent.K2_SetText` (`self.TextRender`) (`self.TextOFF`)))))
        (:`else`)))
    (:`else`)))

(event `self.Interact`
  (bind _pointlight3 (`self.PointLight3`)
    (:`then`
      (if (`SceneComponent.IsVisible` _pointlight3)
        (`SceneComponent.SetVisibility` _pointlight3 false false)
        (`TextRenderComponent.K2_SetText` (`self.TextRender`) (`self.TextOFF`))
        (else
          (`SceneComponent.SetVisibility` _pointlight3 true false)
          (`TextRenderComponent.K2_SetText` (`self.TextRender`) (`self.TextON`))))
      (`self.SwitchActivated`))
    (:`else`)))

(fn `UserConstructionScript`)