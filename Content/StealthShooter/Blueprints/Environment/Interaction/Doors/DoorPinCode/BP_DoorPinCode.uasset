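; BP_DoorPinCode is a PIN code door interactable for the stealth shooter.
; Its Interact event creates a WBP_PinCodeWidget, adds it to the viewport, switches the player to UI-only input focused on the widget and shows the mouse cursor.
; GetCorrectPin exposes the stored CorrectPin; this graph contains no code checking or door-opening logic.
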(event `/Game/StealthShooter/Blueprints/Interfaces/BPI_Interactable.Interact`
  (bind _returnvalue (`GameplayStatics.GetPlayerController` 0))
  (bind _returnvalue_2 (`|CreateWidget` "/Game/StealthShooter/Blueprints/Environment/Interaction/Doors/DoorPinCode/Widgets/WBP_PinCodeWidget.WBP_PinCodeWidget_C"))
  (bind _output_get (set `self.PinWidget` _returnvalue_2))
  (`UserWidget.AddToViewport` _output_get 0)
  (`WidgetBlueprintLibrary.SetInputMode_UIOnlyEx` _returnvalue _output_get "DoNotLock" true)
  (set `PlayerController.bShowMouseCursor` true _returnvalue))

(fn `GetCorrectPin`
  (returns (CorrectPin :type "Array of Integer"))
  (return (`self.CorrectPin`)))

(fn `UserConstructionScript`
  (`parent.UserConstructionScript`))