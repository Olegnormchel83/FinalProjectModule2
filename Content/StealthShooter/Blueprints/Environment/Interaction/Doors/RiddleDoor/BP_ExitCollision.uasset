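; BP_ExitCollision is an exit trigger box for the riddle door puzzle that reacts when the player leaves it.
; When an actor carrying the PlayerTag of its Target reference ends overlap with the box, it calls MoveActor on that Target.
; It then destroys itself if the Target's CubesInCont count equals three, so it stops triggering.
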(event `self.Box.OnComponentEndOverlap`
  (params (OverlappedComponent :type "PrimitiveComponent Object Reference") (OtherActor :type "Actor Object Reference") (OtherComp :type "PrimitiveComponent Object Reference") (OtherBodyIndex :type Integer))
  (bind _target (`self.Target`)
    (:`then`
      (if (`self.ActorHasTag` OtherActor (`/Game/StealthShooter/Blueprints/Environment/Interaction/Doors/BP_DoorParent.PlayerTag` _target))
        (`/Game/StealthShooter/Blueprints/Environment/Interaction/Doors/RiddleDoor/BP_RiddleDoor.MoveActor` (`self.Target`))
        (if (== (`/Game/StealthShooter/Blueprints/Environment/Interaction/Doors/RiddleDoor/BP_RiddleDoor.CubesInCont` (`self.Target`)) 3)
          (`self.K2_DestroyActor`))))
    (:`else`)))

(fn `UserConstructionScript`)