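; Puzzle door that sinks in stages as tagged cubes are placed in its arch, then opens.
; Overlaps on Arch2Collision increment a cube count, which the MoveActor event uses to pick one of three timelines that lower the actor, the last drop being the deepest.
; Flags retire each stage when its timeline finishes.
; The final stage enables opening and, if NearPlates is valid, reveals those plates and calls OpenDoor.
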(event `self.Arch2Collision.OnComponentBeginOverlap`
  (params (OverlappedComponent :type "PrimitiveComponent Object Reference") (OtherActor :type "Actor Object Reference") (OtherComp :type "PrimitiveComponent Object Reference") (OtherBodyIndex :type Integer) (bFromSweep :type Boolean) (SweepResult :type "HitResult Structure (by ref)"))
  (if (`self.ActorHasTag` OtherActor (`self.CubeTag`))
    (`/Engine/EditorBlueprintResources/StandardMacros.IncrementInt` (`self.CubesInCont`))))

(event `MoveActor`
  (bind (_returnvalue_x _returnvalue_y _returnvalue_z) (`KismetMathLibrary.BreakVector` (`self.K2_GetActorLocation`)))
  (bind (_returnvalue_x_2 _returnvalue_y_2 _returnvalue_z_2) (`KismetMathLibrary.BreakVector` (`self.K2_GetActorLocation`)))
  (bind (_returnvalue_x_3 _returnvalue_y_3 _returnvalue_z_3) (`KismetMathLibrary.BreakVector` (`self.K2_GetActorLocation`)))
  (bind (_returnvalue_x_4 _returnvalue_y_4 _returnvalue_z_4) (`KismetMathLibrary.BreakVector` (`self.K2_GetActorLocation`)))
  (bind (_returnvalue_x_5 _returnvalue_y_5 _returnvalue_z_5) (`KismetMathLibrary.BreakVector` (`self.K2_GetActorLocation`)))
  (bind (_returnvalue_x_6 _returnvalue_y_6 _returnvalue_z_6) (`KismetMathLibrary.BreakVector` (`self.K2_GetActorLocation`)))
  (switch `int` (`self.CubesInCont`)
    (:`1`
      (if (`self.bCanFirstOffset`)
        (set `self.TargetZOffset` (- _returnvalue_z_3 50.0))
        (bind (_direction _zoffset) (`Timeline|ActorOffset1Cube`)
          (:`Update`
            (`self.K2_SetActorLocation` (`KismetMathLibrary.MakeVector` _returnvalue_x _returnvalue_y (`KismetMathLibrary.MapRangeClamped` _zoffset 0.0 1.0 _returnvalue_z (`self.TargetZOffset`)))))
          (:`Finished`
            (set `self.bCanFirstOffset` false)))))
    (:`2`
      (if (`self.bCanSecondOffset`)
        (set `self.TargetZOffset` (- _returnvalue_z_5 50.0))
        (bind (_direction_2 _zoffset_2) (`Timeline|ActorOffset2Cubes`)
          (:`Update`
            (`self.K2_SetActorLocation` (`KismetMathLibrary.MakeVector` _returnvalue_x_4 _returnvalue_y_4 (`KismetMathLibrary.MapRangeClamped` _zoffset_2 0.0 1.0 _returnvalue_z_4 (`self.TargetZOffset`)))))
          (:`Finished`
            (set `self.bCanSecondOffset` false)))))
    (:`3`
      (if (`self.bCanThirdOffset`)
        (set `self.TargetZOffset` (- _returnvalue_z_2 300.0))
        (bind (_direction_3 _zoffset_3) (`Timeline|ActorOffset3Cubes`)
          (:`Update`
            (`self.K2_SetActorLocation` (`KismetMathLibrary.MakeVector` _returnvalue_x_6 _returnvalue_y_6 (`KismetMathLibrary.MapRangeClamped` _zoffset_3 0.0 1.0 _returnvalue_z_6 (`self.TargetZOffset`)))))
          (:`Finished`
            (set `self.bCanThirdOffset` false)
            (set `self.bCanOpen` true)
            (bind _nearplates (`self.NearPlates`)
              (:`then`
                (`/Game/StealthShooter/Blueprints/Environment/Static/Floor/BP_SideWalk3x3NearRiddleDoor.SetPlatesVisible` _nearplates)
                (`self.OpenDoor`))
              (:`else`))))))))

(fn `UserConstructionScript`
  (`parent.UserConstructionScript`))