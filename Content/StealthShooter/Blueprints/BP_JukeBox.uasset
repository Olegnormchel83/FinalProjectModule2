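; BP_JukeBox is a music manager that switches the Audio component between a home theme and a bunker theme.
; On BeginPlay it binds overlap events on the BP_TimerTrigger and BP_HomeTrigger actors found in the level, then starts the home theme.
; The bunker-entry and return-home handlers stop the current track and restart with the matching theme, without checking which actor overlapped.
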(event `self.ReceiveBeginPlay`
  (bind _returnvalue (`GameplayStatics.GetActorOfClass` "/Game/StealthShooter/Blueprints/Environment/Static/Triggers/BP_TimerTrigger.BP_TimerTrigger_C"))
  (add `self.OnActorBeginOverlap` _returnvalue (`|CreateDelegate` :!event `PlayerEnterTheBunker`))
  (bind _returnvalue_2 (`GameplayStatics.GetActorOfClass` "/Game/StealthShooter/Blueprints/Environment/Static/Triggers/BP_HomeTrigger.BP_HomeTrigger_C"))
  (add `self.OnActorBeginOverlap` _returnvalue_2 (`|CreateDelegate` :!event `PlayerComeBackHome`))
  (bind _audio (`self.Audio`)
    (:`then`
      (bind _hometheme (`self.HomeTheme`)
        (:`then`
          (`AudioComponent.SetSound` _audio _hometheme)
          (`AudioComponent.Play` _audio 0.0))
        (:`else`)))
    (:`else`)))

(event `PlayerEnterTheBunker` :!signature `self.OnActorBeginOverlap`
  (params (OverlappedActor :type "Actor Object Reference") (OtherActor :type "Actor Object Reference"))
  (bind _audio (`self.Audio`)
    (:`then`
      (`AudioComponent.Stop` _audio)
      (bind _bunkertheme (`self.BunkerTheme`)
        (:`then`
          (`AudioComponent.SetSound` _audio _bunkertheme)
          (`AudioComponent.Play` _audio 0.0))
        (:`else`)))
    (:`else`)))

(event `PlayerComeBackHome` :!signature `self.OnActorBeginOverlap`
  (params (OverlappedActor :type "Actor Object Reference") (OtherActor :type "Actor Object Reference"))
  (bind _audio (`self.Audio`)
    (:`then`
      (`AudioComponent.Stop` _audio)
      (bind _hometheme (`self.HomeTheme`)
        (:`then`
          (`AudioComponent.SetSound` _audio _hometheme)
          (`AudioComponent.Play` _audio 0.0))
        (:`else`)))
    (:`else`)))

(fn `UserConstructionScript`)