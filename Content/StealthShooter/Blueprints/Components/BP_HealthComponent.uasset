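; BP_HealthComponent tracks its owner's health in the stealth shooter and signals when the owner dies.
; Health starts at MaxHealth on BeginPlay, and IncreaseHealth and DecreaseHealth change it, clamped between zero and the maximum.
; DecreaseHealth fires the OwnerDied dispatcher before updating Health whenever the hit would bring it to zero or below, with no guard against repeat calls.
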(event `self.ReceiveBeginPlay`
  (set `self.Health` (`self.MaxHealth`)))

(fn `DecreaseHealth`
  (params (InHealth :type "Float (double-precision)"))
  (bind _returnvalue (- (`self.Health`) InHealth))
  (if (<= _returnvalue 0.0)
    (`self.OnOwnerDied`))
  (set `self.Health` (`KismetMathLibrary.FClamp` _returnvalue 0.0 (`self.MaxHealth`))))

(fn `IncreaseHealth`
  (params (InHealth :type "Float (double-precision)"))
  (set `self.Health` (`KismetMathLibrary.FClamp` (+ InHealth (`self.Health`)) 0.0 (`self.MaxHealth`))))