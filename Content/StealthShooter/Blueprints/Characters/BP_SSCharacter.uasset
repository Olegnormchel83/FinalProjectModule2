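; BP_SSCharacter is the stealth shooter character Blueprint, handling damage and death.
; On BeginPlay it binds to its health component's death delegate and its own damage event, which forwards damage to that component.
; Death sets IsDead, disables input through player controller 0, and turns off spring arm and capsule collision.
; The mesh then ragdolls with physics, and the actor expires after a short lifespan.
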(event `self.ReceiveBeginPlay`
  (bind _bp_healthcomponent (`self.BP_HealthComponent`)
    (:`then`
      (add `/Game/StealthShooter/Blueprints/Components/BP_HealthComponent.OnOwnerDied` _bp_healthcomponent (`|CreateDelegate` :!event `Dead`))
      (add `self.OnTakeAnyDamage` (`|CreateDelegate` :!event `OnTakeAnyDamage_Event`)))
    (:`else`)))

(event `OnTakeAnyDamage_Event` :!signature `self.OnTakeAnyDamage`
  (params (DamagedActor :type "Actor Object Reference") (Damage :type "Float (single-precision)") (DamageType :type "DamageType Object Reference") (InstigatedBy :type "Controller Object Reference") (DamageCauser :type "Actor Object Reference"))
  (bind _bp_healthcomponent (`self.BP_HealthComponent`)
    (:`then`
      (`/Game/StealthShooter/Blueprints/Components/BP_HealthComponent.DecreaseHealth` _bp_healthcomponent Damage))
    (:`else`)))

(event `Dead`
  (bind _mesh (`self.Mesh`))
  (set `self.IsDead` true)
  (`self.DisableInput` (`GameplayStatics.GetPlayerController` 0) null)
  (set `SpringArmComponent.bDoCollisionTest` false (`self.SpringArm`))
  (`PrimitiveComponent.SetCollisionEnabled` (`self.CapsuleComponent`) "NoCollision")
  (`PrimitiveComponent.SetCollisionEnabled` _mesh "QueryAndPhysics")
  (`PrimitiveComponent.SetSimulatePhysics` _mesh true)
  (`self.SetLifeSpan` 2.0))

(fn `UserConstructionScript`)