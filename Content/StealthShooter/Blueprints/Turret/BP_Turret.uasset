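; Automated turret that sweeps for the player and fires on detection.
; A timeline swings the mesh back and forth across 180 degrees of yaw while Tick runs a forward line trace for the player tag, accepting only the first hit.
; On detection it switches to Shooting, turning toward the player as a looping timer applies direct damage with muzzle effects.
; Losing the trace clears the timer and resumes patrol from the current rotation toward a random endpoint.
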(event `self.ReceiveBeginPlay`
  (bind _output_get (set `self.StartRotation` (`SceneComponent.K2_GetComponentRotation` (`self.SkeletalMesh`))))
  (bind _output_get_2 (set `self.EndRotation` (`KismetMathLibrary.MakeRotator` (.roll _output_get) (.pitch _output_get) (+ (.yaw _output_get) 180.0))))
  (set `self.TargetRotation` _output_get_2)
  (set `self.CurrentRotation` (`self.StartRotation`))
  (`self.StartPatrol`))

(event `StartPatrol`
  (bind (_direction _rotatetrack) (`Timeline|TurretPatrol` :!via `PlayFromStart` :!label _label)
    (:`Update`
      (`SceneComponent.K2_SetWorldRotation` (`self.SkeletalMesh`) (`KismetMathLibrary.RLerp` (`self.CurrentRotation`) (`self.TargetRotation`) _rotatetrack) false false))
    (:`Finished`
      (switch `ETimelineDirection` (`self.DirectionMove`)
        (:`Forward`
          (set `self.DirectionMove` "Backward")
          (set `self.TargetRotation` (`self.StartRotation`))
          (set `self.CurrentRotation` (`self.EndRotation`)))
        (:`Backward`
          (set `self.DirectionMove` "Forward")
          (set `self.TargetRotation` (`self.EndRotation`))
          (set `self.CurrentRotation` (`self.StartRotation`))))
      (`self.StartPatrol`))))

(event `StopPatrol`
  (goto _label :!via `Stop`))

(event `self.ReceiveTick`
  (params (DeltaSeconds :type "Float (single-precision)"))
  (bind _skeletalmesh (`self.SkeletalMesh`))
  (bind _firetimerhandle (`self.FireTimerHandle`))
  (bind (_returnvalue_roll _returnvalue_pitch _returnvalue_yaw) (`KismetMathLibrary.BreakRotator` (`SceneComponent.K2_GetComponentRotation` _skeletalmesh)))
  (bind (_returnvalue_roll_2 _returnvalue_pitch_2 _returnvalue_yaw_2) (`KismetMathLibrary.BreakRotator` (`KismetMathLibrary.FindLookAtRotation` (`SceneComponent.K2_GetComponentLocation` (`self.SkeletalMesh`)) (`self.K2_GetActorLocation` (`GameplayStatics.GetPlayerCharacter` 0)))))
  (switch `/Game/StealthShooter/Blueprints/Enums/E_TurretState` (`self.CurrentState`)
    (:`NewEnumerator0`
      (bind (_isplayerfind _hitactor) (`self.PlayerSearch`))
      (if _isplayerfind
        (`/Engine/EditorBlueprintResources/StandardMacros.IsValid` _hitactor
          (:`Is Valid`
            (set `self.Player` _hitactor)
            (`self.StopPatrol`)
            (set `self.CurrentState` "NewEnumerator1"))
          (:`Is Not Valid`
            (set `self.Player` null)))))
    (:`NewEnumerator1`
      (`SceneComponent.K2_SetWorldRotation` _skeletalmesh (`KismetMathLibrary.RInterpTo` (`KismetMathLibrary.MakeRotator` _returnvalue_roll _returnvalue_pitch _returnvalue_yaw) (`KismetMathLibrary.MakeRotator` _returnvalue_roll _returnvalue_pitch (- _returnvalue_yaw_2 180.0)) (`GameplayStatics.GetWorldDeltaSeconds`)) false false)
      (`|ExecutionSequence`
        (:`then_0`
          (if (not (`self.bIsStartShoot`))
            (`self.StartShoot`)
            (set `self.bIsStartShoot` true)))
        (:`then_1`
          (bind _isplayerfind_2 (`self.PlayerSearch`))
          (if _isplayerfind_2
            _
            (elif (`KismetSystemLibrary.K2_IsValidTimerHandle` _firetimerhandle)
              (`KismetSystemLibrary.K2_ClearAndInvalidateTimerHandle` _firetimerhandle)
              (set `self.bIsStartShoot` false)
              (set `self.CurrentState` "NewEnumerator0")
              (set `self.TargetRotation` (`KismetArrayLibrary.Array_Random` (`|MakeArray` (`self.StartRotation`) (`self.EndRotation`))))
              (set `self.CurrentRotation` (`SceneComponent.K2_GetComponentRotation` (`self.SkeletalMesh`)))
              (if (== (`self.TargetRotation`) (`self.EndRotation`) :`ErrorTolerance` 1.0)
                (set `self.DirectionMove` "Forward")
                (else
                  (set `self.DirectionMove` "Backward")))
              (`self.StartPatrol`))))))))

(event `StartShoot`
  (bind _returnvalue (`KismetSystemLibrary.K2_SetTimerDelegate` (delegate `CallShootFunc`) (`self.AttackSpeed`) true))
  (set `self.FireTimerHandle` _returnvalue)
  (`self.Shot`))

(event `CallShootFunc`
  (`self.Shot`))

(fn `MultiLineTrace`
  (returns (OutHits :type "Array of HitResult Structure"))
  (bind _scene (`self.Scene`))
  (bind _returnvalue (`SceneComponent.K2_GetComponentLocation` _scene))
  (bind _outhits (`KismetSystemLibrary.LineTraceMulti` :`Start` _returnvalue :`End` (+ _returnvalue (* (`SceneComponent.GetForwardVector` _scene) (`self.Distance`))) :`TraceChannel` "TraceTypeQuery3" :`bTraceComplex` true :`DrawDebugType` "ForOneFrame"))
  (return _outhits))

(fn `PlayerSearch`
  (returns (IsPlayerFind :type Boolean) (HitActor :type "Actor Object Reference"))
  (bind _outhits (`self.MultiLineTrace`))
  (if (!= (`KismetArrayLibrary.Array_Length` _outhits) 0)
    (for _array_element _outhits
      (bind (_bblockinghit _binitialoverlap _time _distance _location _impactpoint _normal _impactnormal _physmat _hitactor) (`GameplayStatics.BreakHitResult` _array_element))
      (if (`self.ActorHasTag` _hitactor (`self.PlayerTag`))
        (`|ExecutionSequence`
          (:`then_0`
            (break))
          (:`then_1`
            (return true _hitactor)))
        (else
          (return false null))))
    (else
      (return false null))))

(fn `Shot`
  (bind _returnvalue (`SceneComponent.K2_GetComponentLocation` (`self.Scene`)))
  (bind _player (`self.Player`)
    (:`then`
      (`|ExecutionSequence`
        (:`then_0`
          (`GameplayStatics.PlaySoundAtLocation` "/Game/MilitaryWeapDark/Sound/Rifle/RifleB_Fire_Cue.RifleB_Fire_Cue" _returnvalue (struct) 1.0 1.0 0.0 null null null null)
          (`GameplayStatics.SpawnEmitterAtLocation` "/Game/MilitaryWeapDark/FX/P_AssaultRifle_MuzzleFlash.P_AssaultRifle_MuzzleFlash" _returnvalue))
        (:`then_1`
          (`GameplayStatics.ApplyDamage` _player (`self.Damage`) null self))))
    (:`else`)))

(fn `UserConstructionScript`)