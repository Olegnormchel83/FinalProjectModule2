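; BP_CheckpointDeathRoom is a checkpoint actor that sets the player's respawn point, named for a death room.
; On overlap it runs the parent logic, then checks for an actor tagged Player and a valid SSGameInstance.
; It passes the location and rotation of RespawnBoxCollision to SetCheckpoint with unit scale, so the respawn transform comes from that box.
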(event `self.ReceiveActorBeginOverlap`
  (params (OtherActor :type "Actor Object Reference"))
  (bind (_returnvalue_location _returnvalue_rotation) (`KismetMathLibrary.BreakTransform` (`SceneComponent.K2_GetComponentToWorld` (`self.RespawnBoxCollision`))))
  (`parent.ReceiveActorBeginOverlap` OtherActor)
  (if (`self.ActorHasTag` OtherActor "Player")
    (bind _ssgame_instance (`self.SSGame Instance`)
      (:`then`
        (`/Game/StealthShooter/Core/GameInstance/BP_SSGameInstance.SetCheckpoint` _ssgame_instance (`KismetMathLibrary.MakeTransform` _returnvalue_location _returnvalue_rotation)))
      (:`else`))))

(fn `UserConstructionScript`
  (`parent.UserConstructionScript`))