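; BP_KeyItem is a key pickup actor in the StealthShooter game that destroys itself when taken or interacted with.
; TakeKeyItem forwards to Interact, and OnOwnerOpened enables query-only collision on its Sphere.
; An unconnected setup chain, not run by the empty BeginPlay, would disable that collision, place the key above a random BP_Storage and bind to that storage's OnOpened event.
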(event `self.ReceiveBeginPlay`)

(event `/Game/StealthShooter/Blueprints/Interfaces/BPI_KeyItem.TakeKeyItem`
  (`/Game/StealthShooter/Blueprints/Interfaces/BPI_Interactable.Interact`))

(event `/Game/StealthShooter/Blueprints/Interfaces/BPI_Interactable.Interact`
  (`self.K2_DestroyActor`))

(event `OnOwnerOpened`
  (`PrimitiveComponent.SetCollisionEnabled` (`self.Sphere`) "QueryOnly"))

(fn `UserConstructionScript`)