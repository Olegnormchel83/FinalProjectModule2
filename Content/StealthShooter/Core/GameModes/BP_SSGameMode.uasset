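; Stealth shooter game mode that runs a countdown-to-lose timer and handles player respawns.
; A player overlapping the BP_TimerTrigger destroys it and starts a looping one-second timer, which broadcasts each tick and triggers PlayerLose at zero.
; PlayerWin and PlayerLose broadcast the result and clear the timer.
; RespawnPlayer replaces the cached controller's pawn with a new, possessed BP_SSCharacter, then broadcasts the respawn.
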(event `self.ReceiveBeginPlay`
  (`|ExecutionSequence`
    (:`then_0`
      (bind _asbp_ssplayer_controller (cast `/Game/StealthShooter/Core/PlayerControllers/BP_SSPlayerController` (`GameplayStatics.GetPlayerController` 0)))
      (set `self.SSPlayer Controller` _asbp_ssplayer_controller))
    (:`then_1`
      (bind _returnvalue (`GameplayStatics.GetActorOfClass` "/Game/StealthShooter/Blueprints/Environment/Static/BP_TimerTrigger.BP_TimerTrigger_C"))
      (add `self.OnActorBeginOverlap` _returnvalue (`|CreateDelegate` :!event `PlayerEnterTheBunker`)))))

(event `PlayerEnterTheBunker` :!signature `self.OnActorBeginOverlap`
  (params (OverlappedActor :type "Actor Object Reference") (OtherActor :type "Actor Object Reference"))
  (if (`self.ActorHasTag` OtherActor "Player")
    (`KismetSystemLibrary.PrintString` "Hello")
    (bind _returnvalue (`KismetSystemLibrary.K2_SetTimerDelegate` (delegate `TickSecond`) 1.0 true))
    (set `self.TimerHandle` _returnvalue)
    (`self.K2_DestroyActor` OverlappedActor)))

(event `TickSecond`
  (bind _returnvalue (- (`self.TimerSeconds`) 1.0))
  (if (`KismetMathLibrary.NearlyEqual_FloatFloat` _returnvalue)
    (set `self.TimerSeconds` _returnvalue)
    (`self.OnTimerTick`)
    (`self.PlayerLose`)
    (else
      (set `self.TimerSeconds` _returnvalue)
      (`self.OnTimerTick`))))

(event `PlayerWin`
  (`self.OnPlayerWin`)
  (`KismetSystemLibrary.K2_ClearAndInvalidateTimerHandle` (`self.TimerHandle`)))

(event `PlayerLose`
  (`KismetSystemLibrary.PrintString` "PlayerLose")
  (`self.OnPlayerLose`)
  (`KismetSystemLibrary.K2_ClearAndInvalidateTimerHandle` (`self.TimerHandle`)))

(fn `GetSecondsRemaining`
  (returns (TimerSeconds :type "Float (double-precision)"))
  (return (`self.TimerSeconds`)))

(fn `RespawnPlayer`
  (params (RespawnTransform :type "Transform Structure"))
  (bind _ssplayer_controller (`self.SSPlayer Controller`)
    (:`then`
      (`self.K2_DestroyActor` (`Controller.K2_GetPawn` _ssplayer_controller))
      (bind _returnvalue (`|SpawnActorFromClass` "/Game/StealthShooter/Blueprints/Characters/BP_SSCharacter.BP_SSCharacter_C" RespawnTransform "AdjustIfPossibleButAlwaysSpawn" "MultiplyWithRoot" null null))
      (`Controller.Possess` (`self.SSPlayer Controller`) _returnvalue)
      (`self.OnPlayerRespawned`))
    (:`else`)))

(fn `UserConstructionScript`)