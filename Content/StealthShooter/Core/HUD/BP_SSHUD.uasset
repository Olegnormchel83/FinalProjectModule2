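; BP_SSHUD is the stealth shooter's HUD, switching between game interface, death screen and win screen.
; On BeginPlay it binds to the character's health component death event and the game mode's respawn and win events, then shows the interface.
; Death swaps in the death screen and unbinds the death event; respawn rebinds it and recreates the interface.
; Winning shows the win widget with UI-only input and cursor.
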(event `self.ReceiveBeginPlay`
  (`|ExecutionSequence`
    (:`then_0`
      (`self.BindEvents`))
    (:`then_1`
      (bind _returnvalue (`|CreateWidget` "/Game/StealthShooter/UI/GameInterface/WBP_GameInterface.WBP_GameInterface_C"))
      (bind _output_get (set `self.GameInterface` _returnvalue))
      (`UserWidget.AddToViewport` _output_get 0))))

(event `PlayerDead`
  (bind _gameinterface (`self.GameInterface`)
    (:`then`
      (`Widget.RemoveFromParent` _gameinterface)
      (bind _returnvalue (`|CreateWidget` "/Game/StealthShooter/UI/WBP_DeathScreen.WBP_DeathScreen_C"))
      (bind _output_get (set `self.DeathScreen` _returnvalue))
      (`UserWidget.AddToViewport` _output_get 0)
      (bind _sscharacter (`self.SSCharacter`)
        (:`then`
          (clear `/Game/StealthShooter/Blueprints/Components/BP_HealthComponent.OnOwnerDied` (`/Game/StealthShooter/Blueprints/Characters/BP_SSCharacter.BP_HealthComponent` _sscharacter)))
        (:`else`)))
    (:`else`)))

(event `PlayerRespawned`
  (bind _asbp_sscharacter (cast `/Game/StealthShooter/Blueprints/Characters/BP_SSCharacter` (`GameplayStatics.GetPlayerCharacter` 0)))
  (add `/Game/StealthShooter/Blueprints/Components/BP_HealthComponent.OnOwnerDied` (`/Game/StealthShooter/Blueprints/Characters/BP_SSCharacter.BP_HealthComponent` _asbp_sscharacter) (`|CreateDelegate` :!event `PlayerDead`))
  (bind _deathscreen (`self.DeathScreen`)
    (:`then`
      (`Widget.RemoveFromParent` _deathscreen)
      (bind _returnvalue (`|CreateWidget` "/Game/StealthShooter/UI/GameInterface/WBP_GameInterface.WBP_GameInterface_C"))
      (bind _output_get (set `self.GameInterface` _returnvalue))
      (`UserWidget.AddToViewport` _output_get 0))
    (:`else`)))

(event `OnPlayerWin`
  (bind _returnvalue (`GameplayStatics.GetPlayerController` 0))
  (bind _gameinterface (`self.GameInterface`)
    (:`then`
      (`Widget.RemoveFromParent` _gameinterface)
      (bind _returnvalue_2 (`|CreateWidget` "/Game/StealthShooter/UI/WBP_WinWidget.WBP_WinWidget_C"))
      (`UserWidget.AddToViewport` _returnvalue_2 0)
      (`WidgetBlueprintLibrary.SetInputMode_UIOnlyEx` _returnvalue null)
      (set `PlayerController.bShowMouseCursor` true _returnvalue))
    (:`else`)))

(fn `BindEvents`
  (bind _asbp_sscharacter (cast `/Game/StealthShooter/Blueprints/Characters/BP_SSCharacter` (`GameplayStatics.GetPlayerCharacter` 0)))
  (bind _output_get (set `self.SSCharacter` _asbp_sscharacter))
  (add `/Game/StealthShooter/Blueprints/Components/BP_HealthComponent.OnOwnerDied` (`/Game/StealthShooter/Blueprints/Characters/BP_SSCharacter.BP_HealthComponent` _output_get) (`|CreateDelegate` :!event `PlayerDead`))
  (bind _asbp_ssgame_mode (cast `/Game/StealthShooter/Core/GameModes/BP_SSGameMode` (`GameplayStatics.GetGameMode`)))
  (bind _output_get_2 (set `self.SSGame Mode` _asbp_ssgame_mode))
  (add `/Game/StealthShooter/Core/GameModes/BP_SSGameMode.OnPlayerRespawned` _output_get_2 (`|CreateDelegate` :!event `PlayerRespawned`))
  (add `/Game/StealthShooter/Core/GameModes/BP_SSGameMode.OnPlayerWin` _output_get_2 (`|CreateDelegate` :!event `OnPlayerWin`)))

(fn `UserConstructionScript`)