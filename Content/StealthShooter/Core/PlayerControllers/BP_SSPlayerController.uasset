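; Player controller for the stealth shooter that drives BP_SSCharacter through Enhanced Input: movement, look, jump, clamped spring-arm zoom and interaction.
; UpdateController runs on BeginPlay and Possess, adding the mapping context, caching the pawn and binding its overlap and death events.
; Overlapping BPI_Interactable actors shows a hint widget and enables interaction, with BPI_KeyItem targets also notifying the character.
; Death switches to UI-only input with a cursor; the pause action is an empty stub.
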(event `self.ReceiveBeginPlay`
  (`self.UpdateController`))

(event `EnhancedInput|/Game/StealthShooter/Core/EnhancedInput/Action/IA_SSMove`
  (params (ActionValue :type "Vector2D Structure") (ElapsedSeconds :type "Float (double-precision)") (TriggeredSeconds :type "Float (double-precision)") (InputAction :type "InputAction Object Reference" :default "/Game/StealthShooter/Core/EnhancedInput/Action/IA_SSMove.IA_SSMove"))
  (bind (_returnvalue_roll _returnvalue_pitch _returnvalue_yaw) (`KismetMathLibrary.BreakRotator` (`self.GetControlRotation`)))
  (:`Triggered`
    (bind _character_movement (`self.Character Movement`)
      (:`then`
        (`|ExecutionSequence`
          (:`then_0`
            (`PawnMovementComponent.AddInputVector` _character_movement (* ActionValue_Y (`KismetMathLibrary.GetForwardVector` (`KismetMathLibrary.MakeRotator` 0.0 0.0 _returnvalue_yaw))) false))
          (:`then_1`
            (`PawnMovementComponent.AddInputVector` _character_movement (* ActionValue_X (`KismetMathLibrary.GetRightVector` (`KismetMathLibrary.MakeRotator` _returnvalue_roll 0.0 _returnvalue_yaw))) false))))
      (:`else`))))

(event `EnhancedInput|/Game/StealthShooter/Core/EnhancedInput/Action/IA_SSLook`
  (params (ActionValue :type "Vector2D Structure") (ElapsedSeconds :type "Float (double-precision)") (TriggeredSeconds :type "Float (double-precision)") (InputAction :type "InputAction Object Reference" :default "/Game/StealthShooter/Core/EnhancedInput/Action/IA_SSLook.IA_SSLook"))
  (:`Triggered`
    (`self.AddYawInput` ActionValue_X)
    (`self.AddPitchInput` ActionValue_Y)))

(event `EnhancedInput|/Game/StealthShooter/Core/EnhancedInput/Action/IA_SSJump`
  (params (ActionValue :type Boolean) (ElapsedSeconds :type "Float (double-precision)") (TriggeredSeconds :type "Float (double-precision)") (InputAction :type "InputAction Object Reference" :default "/Game/StealthShooter/Core/EnhancedInput/Action/IA_SSJump.IA_SSJump"))
  (:`Triggered`
    (bind _sscharacter (`self.SSCharacter`)
      (:`then`
        (`Character.Jump` _sscharacter))
      (:`else`)))
  (:`Completed`
    (bind _sscharacter_2 (`self.SSCharacter`)
      (:`then`
        (`Character.StopJumping` _sscharacter_2))
      (:`else`))))

(event `EnhancedInput|/Game/StealthShooter/Core/EnhancedInput/Action/IA_SSPause`
  (params (ActionValue :type Boolean) (ElapsedSeconds :type "Float (double-precision)") (TriggeredSeconds :type "Float (double-precision)") (InputAction :type "InputAction Object Reference" :default "/Game/StealthShooter/Core/EnhancedInput/Action/IA_SSPause.IA_SSPause"))
  (:`Triggered`
    (if (`GameplayStatics.IsGamePaused`)
      _)))

(event `EnhancedInput|/Game/StealthShooter/Core/EnhancedInput/Action/IA_SSCameraScroll`
  (params (ActionValue :type "Float (double-precision)") (ElapsedSeconds :type "Float (double-precision)") (TriggeredSeconds :type "Float (double-precision)") (InputAction :type "InputAction Object Reference" :default "/Game/StealthShooter/Core/EnhancedInput/Action/IA_SSCameraScroll.IA_SSCameraScroll"))
  (:`Triggered`
    (if (> ActionValue 0.0)
      (`self.CameraScrollDown`)
      (else
        (`self.CameraScrollUp`)))))

(event `PlayerDead`
  (`WidgetBlueprintLibrary.SetInputMode_UIOnlyEx` self null)
  (set `self.bShowMouseCursor` true))

(event `CharacterBeginOverlap`
  (params (OverlappedActor :type "Actor Object Reference") (OtherActor :type "Actor Object Reference"))
  (if (`KismetSystemLibrary.DoesImplementInterface` OtherActor "/Game/StealthShooter/Blueprints/Interfaces/BPI_Interactable.BPI_Interactable_C")
    (set `self.bCanInteract` true)
    (set `self.InteractedActor` OtherActor)
    (bind _returnvalue (`|CreateWidget` "/Game/StealthShooter/UI/InteractWidget/WBP_InteractHint.WBP_InteractHint_C"))
    (bind _output_get (set `self.WBP_InteractHint` _returnvalue))
    (`UserWidget.AddToViewport` _output_get 0)))

(event `CharacterEndOverlap`
  (params (OverlappedActor :type "Actor Object Reference") (OtherActor :type "Actor Object Reference"))
  (if (`KismetSystemLibrary.DoesImplementInterface` OtherActor "/Game/StealthShooter/Blueprints/Interfaces/BPI_Interactable.BPI_Interactable_C")
    (set `self.bCanInteract` false)
    (set `self.InteractedActor` null)
    (bind _wbp_interacthint (`self.WBP_InteractHint`)
      (:`then`
        (`Widget.RemoveFromParent` _wbp_interacthint))
      (:`else`))))

(event `EnhancedInput|/Game/StealthShooter/Core/EnhancedInput/Action/IA_SSInteract`
  (params (ActionValue :type Boolean) (ElapsedSeconds :type "Float (double-precision)") (TriggeredSeconds :type "Float (double-precision)") (InputAction :type "InputAction Object Reference" :default "/Game/StealthShooter/Core/EnhancedInput/Action/IA_SSInteract.IA_SSInteract"))
  (:`Triggered`
    (if (`self.bCanInteract`)
      (if (`KismetSystemLibrary.DoesImplementInterface` (`self.InteractedActor`) "/Game/StealthShooter/Blueprints/Interfaces/BPI_KeyItem.BPI_KeyItem_C")
        (message `/Game/StealthShooter/Blueprints/Interfaces/BPI_PlayerActions.TakeKeyItem` (`self.SSCharacter`))
        (message `/Game/StealthShooter/Blueprints/Interfaces/BPI_Interactable.Interact` (`self.InteractedActor`))
        (else
          (message `/Game/StealthShooter/Blueprints/Interfaces/BPI_Interactable.Interact` (`self.InteractedActor`)))))))

(event `self.ReceivePossess`
  (params (PossessedPawn :type "Pawn Object Reference"))
  (`self.UpdateController`))

(fn `CameraScrollDown`
  (bind _mincamerradistance (`self.MinCamerraDistance`))
  (bind _sscharacter (`self.SSCharacter`)
    (:`then`
      (bind _springarm (`/Game/StealthShooter/Blueprints/Characters/BP_SSCharacter.SpringArm` _sscharacter))
      (bind _returnvalue (- (`SpringArmComponent.TargetArmLength` _springarm) (`self.CameraSlideStep`)))
      (if (<= _returnvalue _mincamerradistance)
        (set `SpringArmComponent.TargetArmLength` _mincamerradistance _springarm)
        (else
          (set `SpringArmComponent.TargetArmLength` _returnvalue _springarm))))
    (:`else`)))

(fn `CameraScrollUp`
  (bind _maxcamerradistance (`self.MaxCamerraDistance`))
  (bind _sscharacter (`self.SSCharacter`)
    (:`then`
      (bind _springarm (`/Game/StealthShooter/Blueprints/Characters/BP_SSCharacter.SpringArm` _sscharacter))
      (bind _returnvalue (+ (`SpringArmComponent.TargetArmLength` _springarm) (`self.CameraSlideStep`)))
      (if (>= _returnvalue _maxcamerradistance)
        (set `SpringArmComponent.TargetArmLength` _maxcamerradistance _springarm)
        (else
          (set `SpringArmComponent.TargetArmLength` _returnvalue _springarm))))
    (:`else`)))

(fn `UpdateController`
  (bind _sscharacter (`self.SSCharacter`))
  (`WidgetBlueprintLibrary.SetInputMode_GameOnly` self)
  (set `self.bShowMouseCursor` false)
  (`EnhancedInputSubsystemInterface.AddMappingContext` (subsystem `EnhancedInputLocalPlayerSubsystem`) "/Game/StealthShooter/Core/EnhancedInput/IMC_SS.IMC_SS" 0 (struct))
  (bind _asbp_sscharacter (cast `/Game/StealthShooter/Blueprints/Characters/BP_SSCharacter` (`self.K2_GetPawn`)))
  (bind _output_get (set `self.SSCharacter` _asbp_sscharacter))
  (set `self.Character Movement` (`Character.CharacterMovement` _output_get))
  (add `self.OnActorBeginOverlap` _sscharacter (`|CreateDelegate` :!event `CharacterBeginOverlap`))
  (add `self.OnActorEndOverlap` _sscharacter (`|CreateDelegate` :!event `CharacterEndOverlap`))
  (add `/Game/StealthShooter/Blueprints/Components/BP_HealthComponent.OnOwnerDied` (`/Game/StealthShooter/Blueprints/Characters/BP_SSCharacter.BP_HealthComponent` (`self.SSCharacter`)) (`|CreateDelegate` :!event `PlayerDead`)))

(fn `UserConstructionScript`)